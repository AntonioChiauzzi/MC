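; Weather station actor that can replace its base mesh at runtime with a glTF model loaded from a file path.
; On BeginPlay, when an override path is set, it clears and hides BaseMesh, loads the glTF and walks every scene's root nodes.
; SpawnAllMeshesInNode recursively adds static mesh components for node primitives, attaching all to the actor root with each node's own transform, so parent node transforms are not accumulated.
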(event EventBeginPlay
  (bind _runtimeoverrideassetpath (Variables|Default|GetRuntimeOverrideAssetPath))
  (bind _basemesh (Variables|Default|GetBaseMesh))
  (|CallParentFunction)
  (if (and (Variables|Default|GetbHasAssetOverride) (not (Utilities|Array|IsEmpty _runtimeoverrideassetpath)))
    (Components|StaticMesh|SetStaticMesh _basemesh 0)
    (Rendering|SetVisibility _basemesh false true)
    (bind _returnvalue (Class|GlTFRuntimeFunctionLibrary|GlTFLoadAssetfromFilename _runtimeoverrideassetpath false))
    (for _array_element (Class|GlTFRuntimeAsset|GetScenes _returnvalue)
      (for _array_element_2 (.RootNodesIndices (Utilities|Struct|BreakglTFRuntimeScene _array_element))
        (CallFunction|SpawnAllMeshesinNode _returnvalue _array_element_2)))))

(event Collision|EventActorBeginOverlap
  (params (OtherActor :type Actor%20Object%20Reference)))

(event EventTick
  (params (DeltaSeconds :type Float%20%28single-precision%29)))

(fn ConstructionScript)

(fn SpawnAllMeshesinNode
  (params (GLTFAsset :type Gl%20TF%20Runtime%20Asset%20Object%20Reference) (NodeIndex :type Integer))
  (bind _node (Class|GlTFRuntimeAsset|GetNode GLTFAsset NodeIndex))
  (bind (_index _name _transform _meshindex _skinindex _cameraindex _childrenindices) (Utilities|Struct|BreakglTFRuntimeNode _node))
  (if (>= _meshindex 0)
    (bind _returnvalue (Class|GlTFRuntimeAsset|LoadStaticMeshesfromPrimitives GLTFAsset _meshindex))
    (for _array_element _returnvalue
      (bind _returnvalue_2 (AddComponent|AddStaticMeshComponent false))
      (Components|StaticMesh|SetStaticMesh _returnvalue_2 _array_element)
      (Transformation|AttachComponentToComponent _returnvalue_2 (Variables|Transformation|GetRootComponent) "None" "KeepRelative" "KeepRelative" "KeepRelative" true)
      (Transformation|SetRelativeTransform _returnvalue_2 _transform false false)))
  (for _array_element_2 _childrenindices
    (CallFunction|SpawnAllMeshesinNode GLTFAsset _array_element_2)))