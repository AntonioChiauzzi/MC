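; BP_DynamicPawn is a pawn that takes its appearance from a glTF model loaded at runtime.
; On BeginPlay it reads the saved file path from MCGameInstance and, if not empty, loads that file as an absolute path via glTFRuntime.
; It puts the first primitive of mesh 0 on MeshComponent as a static mesh, then calls ApplyAutoScalingToMesh, which is defined outside this graph.
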(event EventBeginPlay
  (bind _asmcgame_instance (Utilities|Casting|CastToMCGameInstance (Game|GetGameInstance)))
  (if (not (Utilities|Array|IsEmpty (Variables|/Script/MC.MCGameInstance|GetSavedDynamicGltfPath _asmcgame_instance)))
    (bind _returnvalue (Class|GlTFRuntimeFunctionLibrary|GlTFLoadAssetfromFilename (Variables|/Script/MC.MCGameInstance|GetSavedDynamicGltfPath _asmcgame_instance) false))
    (bind _returnvalue_2 (Class|GlTFRuntimeAsset|LoadStaticMeshesfromPrimitives _returnvalue))
    (Components|StaticMesh|SetStaticMesh (Variables|Default|GetMeshComponent) (Utilities|Array|Get(acopy) _returnvalue_2))
    (Class|DynamicPawn|ApplyAutoScalingtoMesh)))

(event Collision|EventActorBeginOverlap
  (params (OtherActor :type Actor%20Object%20Reference)))

(event EventTick
  (params (DeltaSeconds :type Float%20%28single-precision%29)))

(fn ConstructionScript)